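; Actor that plays OVR LipSync narration for a SlideActor presentation, driving skeletal mesh morph targets from visemes.
; Construction script finds the SlideActor through a box overlap and copies its slide sounds and times.
; A paused timer, released once the presentation starts, launches the first slide.
; Tick then uses a timer or per-slide Delay to play the current slide's audio and lip-sync sequence, without advancing the index.
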(event OnVisemesReady(OVRLipSyncPlayback)
  (Class|OVRLipSyncActorComponentBase|AssignVisemestoMorphTargets (Variables|Default|GetOVRLipSyncPlayback) (Variables|SkeletalMeshActor|GetSkeletalMeshComponent)))

(event EventBeginPlay
  (bind _slideactor (Variables|Default|GetSlideActor))
  (Class|SlideActor|SetBoolIsUsingOVRLipSync _slideactor)
  (Class|SlideActor|SetSlideIndex _slideactor -1)
  (bind _returnvalue (Utilities|Time|SetTimerbyFunctionName 0 "FirstSlidePlayback" 3.68))
  (bind _output_get (Variables|Default|SetFirstSlideTimerHandle _returnvalue))
  (Utilities|Time|PauseTimerbyHandle _output_get))

(event EventTick
  (params (DeltaSeconds :type Float%20%28single-precision%29))
  (bind _slideactor (Variables|Default|GetSlideActor))
  (bind _ovrlipsyncplayback (Variables|Default|GetOVRLipSyncPlayback))
  (Utilities|IsValid _slideactor
    (:Is%20Valid
      (bind _returnvalue (Class|SlideActor|GetBoolIsStarted _slideactor))
      (if _returnvalue
        (bind _returnvalue_2 (Class|SlideActor|GetSlideIndex _slideactor))
        (if (< _returnvalue_2 0)
          (Utilities|Time|UnpauseTimerbyHandle (Variables|Default|GetFirstSlideTimerHandle))
          (elif (Math|Float|NearlyEqual(Float) (Utilities|Time|GetTimerRemainingTimebyHandle (Variables|Default|GetSlideTimerHandle)) 0.0 1e-06)
            (bind _returnvalue_3 (Utilities|Time|SetTimerbyFunctionName 0 "PresentationPlayback" 3.6))
            (Variables|Default|SetSlideTimerHandle _returnvalue_3)
            (else
              (Utilities|FlowControl|Delay (+ (Utilities|Array|Get(acopy) (Variables|Default|GetSlideTimeArray) _returnvalue_2) 3.95))
              (Class|OVRLipSyncPlaybackActorComponent|SetAudioComponent _ovrlipsyncplayback (Utilities|Array|Get(acopy) (Variables|Default|GetSoundArray) _returnvalue_2))
              (Class|OVRLipSyncPlaybackActorComponent|Start _ovrlipsyncplayback (Variables|Default|GetAudio) (Utilities|Array|Get(acopy) (Variables|Default|GetSequenceArray) _returnvalue_2)))))))))

(fn ConstructionScript
  (bind _box (Variables|Default|GetBox))
  (bind _outcomponents (Collision|BoxOverlapComponents (Transformation|GetWorldLocation _box) (Variables|/Script/Engine.BoxComponent|GetBoxExtent _box) (Variables|Default|GetObject%20Types) "/Script/Engine.BoxComponent" 0 :!class /Script/Engine.KismetSystemLibrary))
  (for _array_element _outcomponents
    (bind _asslide_actor (Utilities|Casting|CastToSlideActor (Components|GetOwner _array_element)))
    (bind _output_get (Variables|Default|SetSlideActor _asslide_actor))
    (bind (_inslidetimes _inslidesounds) (Class|SlideActor|GetSoundData _output_get))
    (Variables|Default|SetSoundArray _inslidesounds)
    (Variables|Default|SetSlideTimeArray _inslidetimes)))

(fn SlideIndex++
  (params (LastIndex :type Integer))
  (bind _slideindex (Variables|Default|GetSlideIndex))
  (if (<= _slideindex LastIndex)
    (bind _result (Math|Integer|IncrementInt _slideindex)
      (:%20%20
        (return _result)))))

(fn FirstSlidePlayback
  (bind _ovrlipsyncplayback (Variables|Default|GetOVRLipSyncPlayback))
  (Class|SlideActor|SetSlideIndex (Variables|Default|GetSlideActor))
  (Class|OVRLipSyncPlaybackActorComponent|SetAudioComponent _ovrlipsyncplayback (Utilities|Array|Get(acopy) (Variables|Default|GetSoundArray)))
  (Class|OVRLipSyncPlaybackActorComponent|Start _ovrlipsyncplayback (Variables|Default|GetAudio) (Utilities|Array|Get(acopy) (Variables|Default|GetSequenceArray))))

(fn PresentationPlayback
  (bind _ovrlipsyncplayback (Variables|Default|GetOVRLipSyncPlayback))
  (Development|PrintString "Hello")
  (bind _returnvalue (Class|SlideActor|GetSlideIndex (Variables|Default|GetSlideActor)))
  (Class|OVRLipSyncPlaybackActorComponent|SetAudioComponent _ovrlipsyncplayback (Utilities|Array|Get(acopy) (Variables|Default|GetSoundArray) _returnvalue))
  (Class|OVRLipSyncPlaybackActorComponent|Start _ovrlipsyncplayback (Variables|Default|GetAudio) (Utilities|Array|Get(acopy) (Variables|Default|GetSequenceArray) _returnvalue)))